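; Blueprint function library with shared helpers for game mechanics and player input.
; GetAttributeComponent fetches an actor's attribute component through BPI_MechanicGeneral, returning empty when the actor is invalid or lacks that interface.
; SetInputModeGeneral switches between Game, UI, and Game and UI input modes in one call.
; It then sets the controller's cursor visibility from FlushInput, leaving its ShowMouseCursor parameter unused.
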(fn GetAttributeComponent
  (params (Actor :type Actor%20Object%20Reference))
  (Utilities|IsValid Actor
    (:Is%20Valid
      (bind _asbpi_mechanic_general (Utilities|Casting|CastToBPI_MechanicGeneral Actor)
        (:then
          (bind _returnvalue (Default|GetAttributeComponent _asbpi_mechanic_general))
          (return _returnvalue))
        (:CastFailed
          _)))
    (:Is%20Not%20Valid
      _))
  (return 0))

(fn SetInputModeGeneral
  (params (InputMode :type E_InputMode%20Enum :default "NewEnumerator0") (PlayerController :type Player%20Controller%20Object%20Reference) (InWidgetToFocus :type Widget%20Object%20Reference) (InMouseLockMode :type EMouseLockMode%20Enum :default "DoNotLock") (bHideCursorDuringCapture :type Boolean) (bFlushInput :type Boolean) (bShowMouseCursor :type Boolean))
  (Utilities|FlowControl|Sequence
    (:then_0
      (switch Utilities|FlowControl|Switch|SwitchonE_InputMode InputMode
        (:NewEnumerator0
          (Input|SetInputModeGameOnly PlayerController bFlushInput))
        (:NewEnumerator1
          (Input|SetInputModeUIOnly PlayerController InWidgetToFocus InMouseLockMode bFlushInput))
        (:NewEnumerator2
          (Input|SetInputModeGameandUI PlayerController InWidgetToFocus InMouseLockMode bHideCursorDuringCapture bFlushInput))))
    (:then_1
      (Variables|/Script/Engine.PlayerController|SetbShowMouseCursor PlayerController bFlushInput))))