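; Actor component that stores named gameplay attributes in a map of value, min and max structs.
; Increase and decrease functions clamp the new value to its range, write it back and broadcast specific and generic change events.
; A decrease that brings the designated death attribute to zero or below also fires a death event.
; Getters return raw values or a value-over-max ratio, and BeginPlay broadcasts an initialization event.
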(event EventBeginPlay
  (CallFunction|InitializeAttributeComponent))

(fn DecreaseAttribute
  (params (AttributeName :type Name) (Amount :type Float%20%28double-precision%29))
  (bind _attributes (Variables|AttributeConfig|GetAttributes))
  (bind (_value _returnvalue) (Utilities|Map|Find _attributes AttributeName))
  (if _returnvalue
    (bind _output_get (LocalVariables|SetL_Attributes _value))
    (bind _structout (Utilities|Struct|SetmembersinS_MechanicAttributeValues (LocalVariables|GetL_Attributes) (Math|Float|Clamp(Float) (- (.Value (Utilities|Struct|BreakS_MechanicAttributeValues _output_get)) Amount) (.MinValue (Utilities|Struct|BreakS_MechanicAttributeValues _output_get)) (.MaxValue (Utilities|Struct|BreakS_MechanicAttributeValues _output_get)))))
    (Utilities|Map|Add (Variables|AttributeConfig|GetAttributes) AttributeName _structout)
    (Default|CallOnDecreaseAttribute AttributeName (Utilities|Struct|BreakS_MechanicAttributeValues _structout))
    (Default|CallOnAttributeChanged AttributeName (Utilities|Struct|BreakS_MechanicAttributeValues _structout))
    (if (and (<= (Utilities|Struct|BreakS_MechanicAttributeValues _structout) 0.0) (== AttributeName (Variables|AttributeConfig|GetListenDeathAttribute)))
      (Default|CallOnDeath))))

(fn IncreaseAttribute
  (params (AttributeName :type Name) (Amount :type Float%20%28double-precision%29))
  (bind _attributes (Variables|AttributeConfig|GetAttributes))
  (bind (_value _returnvalue) (Utilities|Map|Find _attributes AttributeName))
  (if _returnvalue
    (bind _output_get (LocalVariables|SetL_Attributes _value))
    (bind _structout (Utilities|Struct|SetmembersinS_MechanicAttributeValues (LocalVariables|GetL_Attributes) (Math|Float|Clamp(Float) (+ (.Value (Utilities|Struct|BreakS_MechanicAttributeValues _output_get)) Amount) (.MinValue (Utilities|Struct|BreakS_MechanicAttributeValues _output_get)) (.MaxValue (Utilities|Struct|BreakS_MechanicAttributeValues _output_get)))))
    (Utilities|Map|Add (Variables|AttributeConfig|GetAttributes) AttributeName _structout)
    (Default|CallOnIncreaseAttribute AttributeName (Utilities|Struct|BreakS_MechanicAttributeValues _structout))
    (Default|CallOnAttributeChanged AttributeName (Utilities|Struct|BreakS_MechanicAttributeValues _structout))))

(fn GetAttributeValues
  (params (AttributeName :type Name))
  (bind _attributes (Variables|AttributeConfig|GetAttributes))
  (bind (_value _returnvalue) (Utilities|Map|Find _attributes AttributeName))
  (bind (_value_2 _minvalue _maxvalue) (Utilities|Struct|BreakS_MechanicAttributeValues _value))
  (if _returnvalue
    (return _value_2 _minvalue _maxvalue)))

(fn GetAttributeNormal
  (params (AttributeName :type Name))
  (bind _attributes (Variables|AttributeConfig|GetAttributes))
  (bind (_value _returnvalue) (Utilities|Map|Find _attributes AttributeName))
  (bind (_value_2 _maxvalue) (Utilities|Struct|BreakS_MechanicAttributeValues _value))
  (if _returnvalue
    (return (/ _value_2 _maxvalue))))

(fn InitializeAttributeComponent
  (Default|CallOnInitializeAttributeComponent))