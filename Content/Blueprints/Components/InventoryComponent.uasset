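; InventoryComponent is an inventory component that creates and stores item objects for its owning actor.
; TryAddItem constructs an item from a class with the owner as outer, adds it to Items, then initializes it with the inventory, owning actor, character and player controller.
; FindItemByClass scans Items and returns the first exact class match.
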(event EventBeginPlay)

(event EventTick
  (params (DeltaSeconds :type Float%20%28single-precision%29)))

(fn TryAddItem
  (params (ItemClass :type Base%20Item%20Class%20Reference))
  (bind _returnvalue (Components|GetOwner))
  (bind _ascharacter (Utilities|Casting|CastToCharacter _returnvalue))
  (bind _returnvalue_2 (Game|ConstructObjectfromClass (Components|GetOwner) ItemClass))
  (Utilities|Array|AddUnique (Variables|Default|GetItems) _returnvalue_2)
  (Default|InitializeItem _returnvalue_2 self (Components|GetOwner) _ascharacter (.AsPlayer%20Controller (Utilities|Casting|CastToPlayerController (Pawn|GetController _ascharacter)))))

(fn FindItembyClass
  (params (ItemClass :type Base%20Item%20Class%20Reference))
  (bind _array_element (Utilities|Array|ForEachLoopwithBreak (Variables|Default|GetItems) :!label _label)
    (:LoopBody
      (if (== (Utilities|GetClass _array_element) ItemClass)
        (Utilities|FlowControl|Sequence
          (:then_0
            (goto _label Break))
          (:then_1
            (return _array_element)))))))