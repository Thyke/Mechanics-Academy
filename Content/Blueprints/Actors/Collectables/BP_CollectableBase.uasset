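; BP_CollectableBase is a base actor for collectables that provides shared feedback effects.
; Its SpawnEffects function takes a location, rotation and scale, then spawns optional Niagara and Cascade particle systems and plays an optional sound at that location.
; Each effect is validity-checked separately, so any can be left unset.
; The event graph holds only disabled default events, so pickup logic is not defined here.
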(event EventBeginPlay
  (|CallParentFunction) ; This node is disabled and will not be called.\nDrag off pins to build functionality.
)

(event Collision|EventActorBeginOverlap
  (params (OtherActor :type Actor%20Object%20Reference))
  (|CallParentFunction OtherActor) ; This node is disabled and will not be called.\nDrag off pins to build functionality.
)

(event EventTick
  (params (DeltaSeconds :type Float%20%28single-precision%29))
  (|CallParentFunction DeltaSeconds) ; This node is disabled and will not be called.\nDrag off pins to build functionality.
)

(fn ConstructionScript
  (|CallParentFunction))

(fn SpawnEffects
  (params (Location :type Vector) (Rotation :type Rotator) (Scale :type Vector))
  (Utilities|FlowControl|Sequence
    (:then_0
      (bind _niagaravfx (Variables|CollectableConfig|GetNiagaraVFX)
        (:then
          (Niagara|SpawnSystematLocation _niagaravfx Location Rotation Scale))
        (:else)))
    (:then_1
      (bind _cascadevfx (Variables|CollectableConfig|GetCascadeVFX)
        (:then
          (Effects|SpawnEmitteratLocation _cascadevfx Location Rotation Scale))
        (:else)))
    (:then_2
      (bind _sound (Variables|CollectableConfig|GetSound)
        (:then
          (Audio|PlaySoundatLocation _sound Location "0, 0, 0" 1.0 1.0 0.0 0 0 0 0))
        (:else)))))